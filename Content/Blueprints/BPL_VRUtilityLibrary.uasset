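; BPL_VRUtilityLibrary is a Blueprint function library of helpers for VR interaction with BP_BaseInteractiveItem objects.
; InteractiveItemChangeType casts the old and new targets to interactive items and classifies the transition between them.
; SendOnOverHoverEvents turns that transition into OnOver, OnHover and OnOut calls, passing along status, hit and trigger component.
; A small GetLineEnd helper computes a line's endpoint from start, direction and length.
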(fn GetLineEnd
  (params (LineStart :type Vector) (DirectionNormal :type Vector) (LineLength :type Float%20%28single-precision%29))
  (return (+ LineStart (* DirectionNormal LineLength))))

(fn InteractiveItemChangeType
  (params (Old :type Actor%20Object%20Reference) (New :type Actor%20Object%20Reference))
  ;[1 1 1] Cast inputs to Items and store
  (bind _asbp_base_interactive_item (Utilities|Casting|CastToBP_BaseInteractiveItem Old)
    (:then
      _)
    (:CastFailed
      _))
  (LocalVariables|SetOldItem_L _asbp_base_interactive_item)
  (bind _asbp_base_interactive_item_2 (Utilities|Casting|CastToBP_BaseInteractiveItem New)
    (:then
      _)
    (:CastFailed
      _))
  (LocalVariables|SetNewItem_L _asbp_base_interactive_item_2)
  ;[1 1 1] Were we on an item?
  (Utilities|IsValid (LocalVariables|GetOldItem_L)
    (:Is%20Valid
      ;[1 1 1] Are we now on an item?
      (Utilities|IsValid (LocalVariables|GetNewItem_L)
        (:Is%20Valid
          ;[1 1 1] Are they the same item?
          (if (== (LocalVariables|GetOldItem_L) (LocalVariables|GetNewItem_L))
            ;[1 1 1] Return the correct type
            (return "NewEnumerator2" (LocalVariables|GetOldItem_L) (LocalVariables|GetNewItem_L))
            (else
              (return "NewEnumerator5" (LocalVariables|GetOldItem_L) (LocalVariables|GetNewItem_L)))))
        (:Is%20Not%20Valid
          (return "NewEnumerator3" (LocalVariables|GetOldItem_L) (LocalVariables|GetNewItem_L)))))
    (:Is%20Not%20Valid
      ;[1 1 1] Are we now on an item?
      (Utilities|IsValid (LocalVariables|GetNewItem_L)
        (:Is%20Valid
          (return "NewEnumerator1" (LocalVariables|GetOldItem_L) (LocalVariables|GetNewItem_L)))
        (:Is%20Not%20Valid
          (return "NewEnumerator0" (LocalVariables|GetOldItem_L) (LocalVariables|GetNewItem_L)))))))

(fn SendonOverHoverEvents
  (params (Chnage :type EObjectChangeType%20Enum) (OldItem :type BP%20Base%20Interactive%20Item%20Object%20Reference) (NewItem :type BP%20Base%20Interactive%20Item%20Object%20Reference) (Status :type BPS%20Motion%20Controller%20Status%20Structure) (Hit :type Hit%20Result%20Structure) (TriggerComponent :type BP%20Base%20VR%20Pawn%20Component%20Object%20Reference))
  (LocalVariables|SetOldItem_L OldItem)
  (LocalVariables|SetNewItem_L NewItem)
  (LocalVariables|SetStatus_L Status)
  (LocalVariables|SetHit_L Hit)
  (LocalVariables|SetTriggerComponent_L TriggerComponent)
  (switch Utilities|FlowControl|Switch|SwitchonEObjectChangeType Chnage
    (:NewEnumerator1
      (Default|OnOver (LocalVariables|GetNewItem_L) (LocalVariables|GetStatus_L) (LocalVariables|GetHit_L) (LocalVariables|GetTriggerComponent_L))
      (Default|OnHover (LocalVariables|GetNewItem_L) (LocalVariables|GetStatus_L) (LocalVariables|GetHit_L) (LocalVariables|GetTriggerComponent_L)))
    (:NewEnumerator2
      (Default|OnHover (LocalVariables|GetNewItem_L) (LocalVariables|GetStatus_L) (LocalVariables|GetHit_L) (LocalVariables|GetTriggerComponent_L)))
    (:NewEnumerator3
      (Default|OnOut (LocalVariables|GetOldItem_L) (LocalVariables|GetStatus_L) (LocalVariables|GetHit_L) (LocalVariables|GetTriggerComponent_L)))
    (:NewEnumerator5
      (Default|OnOut (LocalVariables|GetOldItem_L) (LocalVariables|GetStatus_L) (LocalVariables|GetHit_L) (LocalVariables|GetTriggerComponent_L))
      (Default|OnOver (LocalVariables|GetNewItem_L) (LocalVariables|GetStatus_L) (LocalVariables|GetHit_L) (LocalVariables|GetTriggerComponent_L))
      (Default|OnHover (LocalVariables|GetNewItem_L) (LocalVariables|GetStatus_L) (LocalVariables|GetHit_L) (LocalVariables|GetTriggerComponent_L)))))