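; BP_ChaperoneLimits is an actor that displays a mesh sized from the SteamVR chaperone play-area bounds.
; The construction script assigns the limits mesh and material, then stores a dynamic material instance.
; On BeginPlay, ResizeToLimits sets the mesh's world X and Y scale from the first bounds point divided by a fixed factor, keeping Z at one, and prints the result.
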(event EventBeginPlay
  (CallFunction|ResizetoLimits))

(event EventActorBeginOverlap
  (params (OtherActor :type Actor%20Object%20Reference)))

(event EventTick
  (params (DeltaSeconds :type Float%20%28single-precision%29)))

(fn ConstructionScript
  (Components|StaticMesh|SetStaticMesh (Variables|Default|GetChaperoneMesh) (Variables|Default|GetLimitsMesh))
  (Rendering|Material|SetMaterial (Variables|Default|GetChaperoneMesh) 0 (Variables|Default|GetMaterial))
  (bind _returnvalue (Rendering|Material|CreateDynamicMaterialInstance (Variables|Default|GetChaperoneMesh) 0 0 :!class /Script/Engine.PrimitiveComponent))
  (Variables|Default|SetDynamicMaterialInstance _returnvalue))

(fn ResizetoLimits
  (bind _steamvrchaperone (Variables|Default|GetSteamVRChaperone))
  (bind _returnvalue (Class|SteamVRChaperoneComponent|GetBounds _steamvrchaperone))
  (bind _item (Utilities|Array|Get(acopy) _returnvalue))
  (bind _returnvalue_2 (/ _item 5e+01))
  (bind (_x _y) (Math|Vector|BreakVector _returnvalue_2))
  (bind _returnvalue_3 (Math|Vector|MakeVector _x _y 1.0))
  (Transformation|SetWorldScale3D (Variables|Default|GetChaperoneMesh) _returnvalue_3)
  (Development|PrintString (Utilities|String|ToString(Vector) _returnvalue_3)))