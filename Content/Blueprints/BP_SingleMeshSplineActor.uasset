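; Actor that stretches a single configurable mesh and material between the first and last of a list of points.
; Update rebuilds the spline from the world-space Points array, then sets the spline mesh's ends from the end points, with tangents multiplied tenfold.
; The construction script runs Update and tapers the mesh from the Scale variable at the start to unit scale at the end.
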(fn ConstructionScript
  (Components|StaticMesh|SetStaticMesh (Variables|Default|GetSplineMesh) (Variables|Default|GetMesh))
  (Rendering|Material|SetMaterial (Variables|Default|GetSplineMesh) 0 (Variables|Default|GetMaterial))
  (CallFunction|Update)
  (SplineMesh|SetStartScale (Variables|Default|GetSplineMesh) (Variables|Default|GetScale) true :!class /Script/Engine.SplineMeshComponent)
  (SplineMesh|SetEndScale (Variables|Default|GetSplineMesh) "(X=1.000,Y=1.000)" true :!class /Script/Engine.SplineMeshComponent))

(fn UpdateSplinePositions
  (Spline|ClearSplinePoints (Variables|Default|GetSpline))
  (for _array_element (Variables|Default|GetPoints)
    (Spline|AddSplinePoint (Variables|Default|GetSpline) _array_element "World")))

(fn UpdateMeshComponent
  (bind _spline (Variables|Default|GetSpline))
  (bind _returnvalue (Spline|GetNumberOfSplinePoints _spline))
  (bind (_location _tangent) (Spline|GetLocationandTangentatSplinePoint _spline 0 "World"))
  (bind (_location_2 _tangent_2) (Spline|GetLocationandTangentatSplinePoint _spline _returnvalue "World"))
  (SplineMesh|SetStartandEnd (Variables|Default|GetSplineMesh) _location (* _tangent 1e+01) _location_2 (* _tangent_2 1e+01) true :!class /Script/Engine.SplineMeshComponent))

(fn Update
  (CallFunction|UpdateSplinePositions)
  (CallFunction|UpdateMeshComponent))