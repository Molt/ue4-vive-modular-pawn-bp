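; Spline actor that draws a chain of deformed meshes through an array of world-space Points.
; The construction script rebuilds the spline and creates one collisionless, slightly tapered spline mesh per segment under SplineAttachment, using the Mesh and Material variables.
; A separate Update function moves the existing spline points, refits each mesh's endpoints and tangents, and hides surplus segments without rebuilding components.
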(fn ConstructionScript
  (CallFunction|BuildSplineComponent)
  (CallFunction|BuildMeshComponents)
  (CallFunction|Update))

(fn BuildSplineComponent
  (Spline|ClearSplinePoints (Variables|Default|GetSpline))
  (for _array_element (Variables|Spline|GetPoints)
    (Spline|AddSplinePoint (Variables|Default|GetSpline) _array_element "World")))

(fn Update
  (CallFunction|UpdateSplinePositions)
  (CallFunction|UpdateMeshComponents))

(fn BuildMeshComponents
  ;[1 1 1] Destroy all SplineAttachment children (SplineMeshComponents)
  (for _array_element (Components|GetChildrenComponents (Variables|Default|GetSplineAttachment) false)
    (Components|DestroyComponent _array_element))
  ;[1 1 1] Create enough SplineMaterialComponents to cover the spline
  (for _index (range 0 (- (Spline|GetNumberOfSplinePoints (Variables|Default|GetSpline)) 2))
    (bind _returnvalue (AddComponent|AddSplineMeshComponent true))
    ;[1 1 1] Set Mesh, Material and Scale of new component
    (Components|StaticMesh|SetStaticMesh _returnvalue (Variables|Spline|GetMesh))
    (Rendering|Material|SetMaterial _returnvalue 0 (Variables|Spline|GetMaterial))
    (SplineMesh|SetStartScale _returnvalue (Math|Vector2D|MakeVector2D 0.5 0.5) true :!class /Script/Engine.SplineMeshComponent)
    (SplineMesh|SetEndScale _returnvalue (Math|Vector2D|MakeVector2D 0.4 0.4) false :!class /Script/Engine.SplineMeshComponent)
    (Collision|SetCollisionEnabled _returnvalue "NoCollision")
    ;[1 1 1] Attach to SplineAttachment
    (Class|SceneComponent|Attachto _returnvalue (Variables|Default|GetSplineAttachment) "None" "KeepRelativeOffset" false)))

(fn UpdateSplinePositions
  (for (_array_element _array_index) (Variables|Spline|GetPoints)
    (Spline|SetLocationatSplinePoint (Variables|Default|GetSpline) _array_index _array_element "World")))

(fn UpdateMeshComponents
  (bind _spline (Variables|Default|GetSpline))
  ;[1 1 1] Iterate over the SplineMeshComponents in SplineAttachment
  (for (_array_element _array_index) (Components|GetChildrenComponents (Variables|Default|GetSplineAttachment) false)
    (bind _asspline_mesh_component (Utilities|Casting|CastToSplineMeshComponent _array_element))
    (Rendering|SetVisibility _asspline_mesh_component (< _array_index (- (Utilities|Array|Length (Variables|Spline|GetPoints)) 1)) false)
    ;[1 1 1] Update the mesh
    (SplineMesh|SetStartandEnd _asspline_mesh_component (.Location (Spline|GetLocationandTangentatSplinePoint _spline _array_index "World")) (.Tangent (Spline|GetLocationandTangentatSplinePoint _spline _array_index "World")) (.Location (Spline|GetLocationandTangentatSplinePoint _spline (+ _array_index 1) "World")) (.Tangent (Spline|GetLocationandTangentatSplinePoint _spline (+ _array_index 1) "World")) true :!class /Script/Engine.SplineMeshComponent)))