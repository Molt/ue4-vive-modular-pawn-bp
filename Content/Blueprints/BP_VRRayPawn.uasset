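; BP_VRRayPawn is a VR pawn that points at and hovers items with laser rays from both motion controllers.
; Each tick, it reads each controller's status, runs a line trace that draws a colored ray and drives an impact component, red for left and green for right.
; Each hit is passed to a hover handler along with that hand's current hover item.
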(event EventTick
  (params (DeltaSeconds :type Float%20%28single-precision%29))
  (Utilities|FlowControl|Sequence
    (:then_0
      (bind _status (CallFunction|GetMotionControllerStatus (Variables|Default|GetMotionControllerL) 0.0 0.0))
      (bind _hit (CallFunction|PerformandDisplayRayLineTrace _status 1e+03 true "(R=1.000000,G=0.000000,B=0.000000,A=1.000000)" 1.0 (Variables|Default|GetRayImpactL)))
      (CallFunction|HandleRayonOverHover _status _hit (Variables|Default|GetRayHoverItemL) self))
    (:then_1
      (bind _status_2 (CallFunction|GetMotionControllerStatus (Variables|Default|GetMotionControllerR) 0.0 0.0))
      (bind _hit_2 (CallFunction|PerformandDisplayRayLineTrace _status_2 1e+03 true "(R=0.000000,G=1.000000,B=0.000000,A=1.000000)" 1.0 (Variables|Default|GetRayImpactR)))
      (CallFunction|HandleRayonOverHover _status_2 _hit_2 (Variables|Default|GetRayHoverItemR) self))))

(fn ConstructionScript
  (|CallParentFunction))