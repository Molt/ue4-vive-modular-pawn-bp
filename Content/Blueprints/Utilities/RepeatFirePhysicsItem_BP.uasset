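; Utility scene component that repeatedly launches a spawned physics actor from its own world location and rotation, starting at BeginPlay.
; The Fire event calls itself after a retriggerable random delay between configurable minimum and maximum values, forming an endless loop.
; Each shot applies an impulse to the spawned actor's first static mesh component along the forward vector, plus random variance, and prints a debug message.
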(event Custom|Fire
  (bind _returnvalue (Transformation|GetWorldTransform))
  (bind (_location _rotation) (Math|Transform|BreakTransform _returnvalue))
  (Utilities|FlowControl|RetriggerableDelay (Math|Random|RandomFloatinRange (Variables|Fire|GetMinFireDelay) (Variables|Fire|GetMaxFireDelay)))
  (Development|PrintString "FIRE!")
  (bind _returnvalue_2 (Game|SpawnActorfromClass (Variables|Fire|GetSpawnActor) (Math|Transform|MakeTransform _location _rotation) "Undefined" 0 0))
  (Physics|AddImpulse (Utilities|Array|Get(acopy) (Actor|GetComponentsByClass _returnvalue_2 "/Script/Engine.StaticMeshComponent")) (+ (* (Math|Vector|GetForwardVector (Transformation|GetWorldRotation)) (Variables|Default|GetForce)) (* (Math|Random|RandomUnitVector) (Math|Random|RandomFloatinRange 0.0 (Variables|Fire|GetForceVariance)))) "None" false)
  (CallFunction|Fire))

(event EventBeginPlay
  (CallFunction|Fire))