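; BP_VRLinePathRenderer is a VR path renderer that displays a list of points as a connected polyline.
; Its Draw function takes the points and draws a debug line between each consecutive pair, using the shared Color and Thickness variables.
; It relies on DrawDebugLine rather than mesh or spline components.
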(fn Draw
  (params (Points :type Array%20of%20Vectors))
  (LocalVariables|SetPathItems_L Points)
  (for _index (range 0 (- (Utilities|Array|Length (LocalVariables|GetPathItems_L)) 2))
    (Rendering|Debug|DrawDebugLine (Utilities|Array|Get(acopy) (LocalVariables|GetPathItems_L) _index) (Utilities|Array|Get(acopy) (LocalVariables|GetPathItems_L) (+ _index 1)) (Variables|Default|GetColor) 0.0 (Variables|Default|GetThickness))))