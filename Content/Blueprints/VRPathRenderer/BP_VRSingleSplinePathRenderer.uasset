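; BP_VRSingleSplinePathRenderer is a VR path renderer that displays a set of points through a single-mesh spline actor.
; Draw lazily spawns one BP_SingleMeshSplineActor at the origin with the configured mesh, material and scale, then reuses it, passing new points and calling Update.
; GetEndPoints reduces a point list to its first and last entries.
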(fn GetEndPoints
  (params (Points :type Array%20of%20Vectors))
  (return (Utilities|Array|MakeArray (Utilities|Array|Get(acopy) Points) (Utilities|Array|Get(acopy) Points (Utilities|Array|LastIndex Points)))))

(fn Draw
  (params (Points :type Array%20of%20Vectors))
  (Utilities|IsValid (Variables|Default|GetSplineActor)
    (:Is%20Valid
      _)
    (:Is%20Not%20Valid
      (bind _returnvalue (Game|SpawnActorfromClass "/Game/Blueprints/BP_SingleMeshSplineActor.BP_SingleMeshSplineActor_C" (Math|Transform|MakeTransform "0, 0, 0") "Undefined" 0 (Variables|Spline|GetMesh) (Variables|Spline|GetMaterial) (Variables|Spline|GetScale)))
      (Variables|Default|SetSplineActor _returnvalue)))
  (Variables|/Game/Blueprints/BP_SingleMeshSplineActor.BP_SingleMeshSplineActor_C|SetPoints (Variables|Default|GetSplineActor) Points)
  (Default|Update (Variables|Default|GetSplineActor)))