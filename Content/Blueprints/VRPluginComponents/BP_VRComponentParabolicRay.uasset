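; VR pointer component that casts a parabolic ray from the controller to detect the actor it points at.
; Each tick it computes arc points from controller location and forward vector, using step count, length and droop rate.
; It line-traces segment by segment on Visibility until a hit registers, then updates child components and sends item events for the hit actor.
; OldFunc and BuildLinePoints hold an alternative arc builder with debug drawing, unused by Tick.
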(event EventTick
  (params (DeltaSeconds :type Float%20%28single-precision%29))
  (bind _status (CallFunction|GetControllerStatus))
  (bind (_location _rotator _forward) (Utilities|Struct|BreakBPS_MotionControllerStatus _status))
  (bind _points (CallFunction|CalculateParabola _location _forward (Variables|Default|GetTraceSteps) (Variables|Default|GetTraceLength) (Variables|Default|GetDroopRate) "0, 0,-1.000000"))
  (Variables|Default|SetLinePoints _points)
  (bind _hit (VR|PerformSegmentedLineTrace _status))
  (bind _output_get (Variables|Default|SetHit _hit))
  (CallFunction|UpdateChildComponents)
  (CallFunction|UpdateCurrentItemandSendEvents (.HitActor (Collision|BreakHitResult _output_get))))

(fn BuildLinePoints
  (params (StartPoint :type Vector) (StepCount :type Integer) (InitialNormal :type Vector) (StepLength :type Float%20%28single-precision%29) (StepDroop :type Float%20%28single-precision%29))
  (Utilities|Array|Clear (Variables|Default|GetLinePoints))
  (LocalVariables|SetDroop_L "0, 0, 0")
  (for _index (range 0 StepCount)
    (bind _output_get (LocalVariables|SetDroop_L (+ (* (Math|Vector|MakeVector 0.0 0.0 (* StepDroop -1.0)) _index) (LocalVariables|GetDroop_L))))
    (Utilities|Array|Add (Variables|Default|GetLinePoints) (+ (* (* (Math|Vector|Normalize InitialNormal) StepLength) _index) _output_get StartPoint))))

(fn OldFunc
  (bind _status (CallFunction|GetControllerStatus))
  (bind _linepoints (Variables|Default|GetLinePoints))
  (bind _tracelength (Variables|Default|GetTraceLength))
  (bind _tracesteps (Variables|Default|GetTraceSteps))
  (bind (_location _rotator _forward) (Utilities|Struct|BreakBPS_MotionControllerStatus _status))
  (bind _returnvalue (Math|Conversions|ToFloat(Integer) _tracesteps))
  (bind _returnvalue_2 (/ _tracelength _returnvalue))
  (VR|BuildLinePoints _location (Variables|Default|GetTraceSteps) _forward _returnvalue_2 (* _returnvalue_2 (Variables|Default|GetDroopRate)))
  (for _index (range 1 (Variables|Default|GetTraceSteps))
    (Rendering|Debug|DrawDebugLine (Utilities|Array|Get(acopy) _linepoints (- _index 1)) (Utilities|Array|Get(acopy) _linepoints _index) "(R=1.000000,G=0.000000,B=0.000000,A=1.000000)" 0.0 1.0))
  (return))

(fn PerformSegmentedLineTrace
  (params (Status :type BPS%20Motion%20Controller%20Status%20Structure))
  (CallFunction|InitPathPointsatStatusLocation Status)
  (for _index (range 0 (- (Utilities|Array|Length (Variables|Default|GetLinePoints)) 2))
    (bind _outhit (Collision|LineTraceByChannel (Utilities|Array|Get(acopy) (Variables|Default|GetLinePoints) _index) (Utilities|Array|Get(acopy) (Variables|Default|GetLinePoints) (+ _index 1)) "TraceTypeQuery1" true 0 "None"))
    (bind _blockinghit (CallFunction|AddHittoPathPoints _outhit))
    (if _blockinghit
      (return _outhit)))
  (return ""))