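; BP_VRComponentProjectileRay is a VR component Blueprint for a projectile ray that visualizes line traces as debug lines.
; DrawRayLineTrace takes a hit result and draws from the trace start to the hit location, or to the trace end when nothing blocks it.
; Each line uses TraceThickness and a color from a random unit vector, leaving TraceColor unused, and the function always returns false.
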(event EventBeginPlay
  (|CallParentFunction))

(event EventTick
  (params (DeltaSeconds :type Float%20%28single-precision%29))
  (|CallParentFunction 0.0))

(fn DrawRayLineTrace
  (params (Hit :type Hit%20Result%20Structure))
  (bind _returnvalue (Math|Random|RandomUnitVector))
  (bind (_bblockinghit _binitialoverlap _time _location _impactpoint _normal _impactnormal _physmat _hitactor _hitcomponent _hitbonename _hititem _tracestart _traceend) (Collision|BreakHitResult Hit))
  (bind _tracethickness (Variables|Default|GetTraceThickness))
  (bind _returnvalue_2 (Math|Conversions|ToLinearColor(Vector) _returnvalue))
  (if _bblockinghit
    (Rendering|Debug|DrawDebugLine _tracestart _location _returnvalue_2 0.0 _tracethickness)
    (else
      (Rendering|Debug|DrawDebugLine _tracestart _traceend _returnvalue_2 0.0 _tracethickness)))
  (return false))