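; VR pointer ray component that traces from the controller each tick to find the interactive item being pointed at.
; A Visibility line trace along the controller's forward optionally draws a debug line and moves the first child component to the impact point, hiding it without a hit.
; The hit actor is compared with the current BP_BaseInteractiveItem to classify the change, which is only printed with the item's name.
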(event EventTick
  (params (DeltaSeconds :type Float%20%28single-precision%29))
  (bind _status (CallFunction|GetControllerStatus))
  (bind _hit (VR|PerformandDisplayLineTrace _status))
  (bind (_change _olditem _newitem) (VR|UpdateCurrentItem _status _hit (Variables|VR|GetCurrentItem)))
  (Development|PrintString (Utilities|String|ToString(Text) (Utilities|Text|FormatText "{c}: {name}" (Utilities|Text|ToText(String) (Utilities|String|EnumtoString _change)) (Utilities|Text|ToText(String) (Utilities|GetDisplayName _newitem))))))

(fn PerformandDisplayLineTrace
  (params (Status :type BPS%20Motion%20Controller%20Status%20Structure))
  (bind _hit (VR|PerformRayLineTrace Status))
  (if (Variables|VR|GetDrawTrace)
    (VR|DrawRayLineTrace _hit))
  (VR|PositionChildComponentatImpact _hit)
  (return _hit))

(fn PerformRayLineTrace
  (params (Status :type BPS%20Motion%20Controller%20Status%20Structure))
  (bind (_location _rotator _forward) (Utilities|Struct|BreakBPS_MotionControllerStatus Status))
  (bind _outhit (Collision|LineTraceByChannel _location (CallFunction|GetLineEnd _location _forward (Variables|VR|GetTraceLength)) "TraceTypeQuery1" true 0 "None"))
  (return _outhit))

(fn DrawRayLineTrace
  (params (Hit :type Hit%20Result%20Structure))
  (bind (_bblockinghit _binitialoverlap _time _location _impactpoint _normal _impactnormal _physmat _hitactor _hitcomponent _hitbonename _hititem _tracestart _traceend) (Collision|BreakHitResult Hit))
  (bind _tracecolor (Variables|VR|GetTraceColor))
  (bind _tracethickness (Variables|VR|GetTraceThickness))
  (if _bblockinghit
    (Rendering|Debug|DrawDebugLine _tracestart _location _tracecolor 0.0 _tracethickness)
    (else
      (Rendering|Debug|DrawDebugLine _tracestart _traceend _tracecolor 0.0 _tracethickness))))

(fn PositionChildComponentatImpact
  (params (Hit :type Hit%20Result%20Structure))
  (bind (_bblockinghit _binitialoverlap _time _location _impactpoint) (Collision|BreakHitResult Hit))
  (bind _output_get (LocalVariables|SetChildComponent (Components|GetChildComponent 0)))
  (Utilities|IsValid _output_get
    (:Is%20Valid
      (Rendering|SetVisibility (LocalVariables|GetChildComponent) _bblockinghit false)
      (if _bblockinghit
        (Transformation|SetWorldLocation (LocalVariables|GetChildComponent) _impactpoint false false)))))

(fn UpdateCurrentItem
  (params (Status :type BPS%20Motion%20Controller%20Status%20Structure) (Hit :type Hit%20Result%20Structure) (CurrentItem :type BP%20Base%20Interactive%20Item%20Object%20Reference%20%28by%20ref%29))
  (LocalVariables|SetOldItem_L CurrentItem)
  (bind _asbp_base_interactive_item (Utilities|Casting|CastToBP_BaseInteractiveItem (.HitActor (Collision|BreakHitResult Hit)))
    (:then
      _)
    (:CastFailed
      _))
  (bind _asbp_base_interactive_item_2 (Utilities|Casting|CastToBP_BaseInteractiveItem (.OldObject (CallFunction|InteractiveItemChangeType (LocalVariables|GetOldItem_L) _asbp_base_interactive_item)))
    (:then
      _)
    (:CastFailed
      _))
  (bind _asbp_base_interactive_item_3 (Utilities|Casting|CastToBP_BaseInteractiveItem (.NewObject (CallFunction|InteractiveItemChangeType (LocalVariables|GetOldItem_L) _asbp_base_interactive_item)))
    (:then
      _)
    (:CastFailed
      _))
  (bind _output_get (Variables|VR|SetCurrentItem _asbp_base_interactive_item_3))
  (return (.Change (CallFunction|InteractiveItemChangeType (LocalVariables|GetOldItem_L) _asbp_base_interactive_item)) _asbp_base_interactive_item_2 _asbp_base_interactive_item_3 _output_get))