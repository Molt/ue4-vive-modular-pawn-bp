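; BP_VRMotionController is a VR motion controller that relays trigger input to BP_BaseVRPawnComponent components beneath it.
; SendMotionControllerInputEvents rebuilds that child list on each call and prints previous and current trigger states.
; Pressed, held and released handlers forward to every listed subcomponent.
; The branch comparing LastStatus with Status to fire those handlers is disconnected, so this function currently dispatches no trigger events.
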(fn SendMotionControllerInputEvents
  (CallFunction|UpdateVRSubcomponents)
  (Development|PrintString (Utilities|String|ToString(Text) (Utilities|Text|FormatText "{was} / {is}" (Utilities|Text|ToText(Boolean) (.TriggerDown (Utilities|Struct|BreakBPS_MotionControllerStatus (Variables|VR|GetLastStatus)))) (Utilities|Text|ToText(Boolean) (.TriggerDown (Utilities|Struct|BreakBPS_MotionControllerStatus (Variables|VR|GetStatus))))))))

(fn OnTriggerPressed
  (for _array_element (Variables|Default|GetVRSubcomponents)
    (Default|OnTriggerPressed _array_element)))

(fn OnTriggerHeld
  (for _array_element (Variables|Default|GetVRSubcomponents)
    (Default|OnTriggerHeld _array_element)))

(fn OnTriggerReleased
  (for _array_element (Variables|Default|GetVRSubcomponents)
    (Default|OnTriggerReleased _array_element)))

(fn UpdateVRSubcomponents
  (Utilities|Array|Clear (Variables|Default|GetVRSubcomponents))
  (for _array_element (Components|GetChildrenComponents true)
    (bind _asbp_base_vrpawn_component (Utilities|Casting|CastToBP_BaseVRPawnComponent _array_element))
    (Utilities|Array|Add (Variables|Default|GetVRSubcomponents) _asbp_base_vrpawn_component)))